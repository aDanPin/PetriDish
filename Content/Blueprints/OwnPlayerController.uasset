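; Player controller that shows the mouse cursor and lets the player dash the controlled MainCellBP toward the point under the cursor.
; IA_Dash traces under the cursor, caches the hit and pushes the cell's Capsule with a physics force aimed from its Edro component.
; Input is then disabled for a one-second delay as a cooldown.
; Pressing stops movement, and a short release or cancel calls SimpleMoveToLocation to the cached point.
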(event Input|EnhancedActionEvents|EnhancedInputActionIA_Dash
  (params (ActionValue :type Boolean) (ElapsedSeconds :type Float%20%28double-precision%29) (TriggeredSeconds :type Float%20%28double-precision%29) (InputAction :type Input%20Action%20Object%20Reference :default "/Game/input/IA_Dash.IA_Dash"))
  (bind (_hit _newparam) (CallFunction|GetLocationUnderCursor))
  (:Triggered
    (if _hit
      (bind _output_get (Variables|Default|SetCachedDestination _newparam))
      (CallFunction|Follow _output_get)
      (Input|DisableInput 0)
      (Utilities|FlowControl|Delay 1.0)
      (Input|EnableInput 0)))
  (:Started
    (AI|Navigation|StopMovement))
  (:Canceled
    (if (< ElapsedSeconds (Variables|Default|GetPressedThreshold)) :!label _label
      (CallFunction|Moveto (Variables|Default|GetCachedDestination))))
  (:Completed
    (goto _label)))

(event Input|EnhancedActionEvents|EnhancedInputActionIA_Dash
  (params (ActionValue :type Boolean) (ElapsedSeconds :type Float%20%28double-precision%29) (TriggeredSeconds :type Float%20%28double-precision%29) (InputAction :type Input%20Action%20Object%20Reference :default "/Game/input/IA_Dash.IA_Dash")))

(event EventBeginPlay
  (bind _returnvalue (PlayerController|LocalPlayerSubsystems|GetEnhancedInputLocalPlayerSubsystem))
  (Variables|Default|SetbShowMouseCursor true)
  (Input|SetInputModeGameandUI 0 0 "DoNotLock" true false)
  (Utilities|IsValid _returnvalue
    (:Is%20Valid
      (Input|AddMappingContext _returnvalue "/Game/Blueprints/IMC_Default.IMC_Default" 0 "(bIgnoreAllPressedKeysUntilRelease=True,bForceImmediately=False,bNotifyUserSettings=False)"))))

(event EventTick
  (params (DeltaSeconds :type Float%20%28single-precision%29)))

(fn ConstructionScript)

(fn GetLocationUnderCursor
  (bind _hitresult (Game|Player|GetHitResultUnderCursorbyChannel "TraceTypeQuery1" true))
  (bind (_bblockinghit _binitialoverlap _time _distance _location) (Collision|BreakHitResult _hitresult))
  (return _bblockinghit _location))

(fn Follow
  (params (Location :type Vector))
  (bind _asmain_cell_bp (Utilities|Casting|CastToMainCellBP (Pawn|GetControlledPawn)))
  (Physics|AddForce (Variables|/Game/Blueprints/MainCellBP.MainCellBP_C|GetCapsule _asmain_cell_bp) (* (Math|Vector|GetUnitDirection(Vector) (Transformation|GetWorldLocation (Variables|/Game/Blueprints/MainCellBP.MainCellBP_C|Getedro _asmain_cell_bp)) Location) 1.5e+04) "None" false)
  (Input|DisableInput 0))

(fn Moveto
  (params (Location :type Vector))
  (AI|Navigation|SimpleMovetoLocation self Location))